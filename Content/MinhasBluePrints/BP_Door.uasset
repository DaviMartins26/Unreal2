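; BP_Door is a swinging door actor that opens and closes through OpenDoor and CloseDoor events.
; A timeline drives the Inside component's relative yaw from 0 to 90 degrees via a lerp, and closing plays it in reverse.
; A Box trigger sets CanBeOpen while a BP_ThirdPersonCharacter overlaps it, though this graph never reads that flag itself.
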(event OnComponentBeginOverlap(Box)
  (params (OverlappedComponent :type Primitive%20Component%20Object%20Reference) (OtherActor :type Actor%20Object%20Reference) (OtherComp :type Primitive%20Component%20Object%20Reference) (OtherBodyIndex :type Integer) (bFromSweep :type Boolean) (SweepResult :type Hit%20Result%20Structure%20%28by%20ref%29))
  (Utilities|Casting|CastToBP_ThirdPersonCharacter OtherActor)
  (Variables|Default|SetCanBeOpen? true))

(event OnComponentEndOverlap(Box)
  (params (OverlappedComponent :type Primitive%20Component%20Object%20Reference) (OtherActor :type Actor%20Object%20Reference) (OtherComp :type Primitive%20Component%20Object%20Reference) (OtherBodyIndex :type Integer))
  (Utilities|Casting|CastToBP_ThirdPersonCharacter OtherActor)
  (Variables|Default|SetCanBeOpen? false))

(event Custom|Open%20Door
  (bind _animacao (Timeline|TimeLine Play)
    (:Update
      (Transformation|SetRelativeRotation (Variables|Default|GetInside) (Math|Rotator|MakeRotator 0.0 0.0 (Math|Float|Lerp 0.0 9e+01 _animacao)) false false))))

(event Custom|Close%20Door
  (bind _animacao (Timeline|TimeLine Reverse)
    (:Update
      (Transformation|SetRelativeRotation (Variables|Default|GetInside) (Math|Rotator|MakeRotator 0.0 0.0 (Math|Float|Lerp 0.0 9e+01 _animacao)) false false))))

(fn ConstructionScript)