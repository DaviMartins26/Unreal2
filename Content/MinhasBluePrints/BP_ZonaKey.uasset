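; BP_ZonaKey is a zone actor that ends the match in victory when the player is inside it.
; Sphere overlap events track the player character's presence and store its reference.
; The Victory event, not triggered within this file, checks that flag, shows the victory HUD, spawns a BP_Bloco, plays a sound and removes key-item widgets.
; It clears the player's IsEnemy flag, then after a delay destroys the player and opens the menu level.
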(event OnComponentBeginOverlap(Sphere)
  (params (OverlappedComponent :type Primitive%20Component%20Object%20Reference) (OtherActor :type Actor%20Object%20Reference) (OtherComp :type Primitive%20Component%20Object%20Reference) (OtherBodyIndex :type Integer) (bFromSweep :type Boolean) (SweepResult :type Hit%20Result%20Structure%20%28by%20ref%29))
  ;[1 1 1] Controle de entrada e saida
  (bind _asbp_third_person_character (Utilities|Casting|CastToBP_ThirdPersonCharacter OtherActor))
  (Variables|Default|SetPlayerInside? true)
  (Variables|Default|SetPlayer%20Ref _asbp_third_person_character))

(event OnComponentEndOverlap(Sphere)
  (params (OverlappedComponent :type Primitive%20Component%20Object%20Reference) (OtherActor :type Actor%20Object%20Reference) (OtherComp :type Primitive%20Component%20Object%20Reference) (OtherBodyIndex :type Integer))
  ;[1 1 1] Controle de entrada e saida
  (Utilities|Casting|CastToBP_ThirdPersonCharacter OtherActor)
  (Variables|Default|SetPlayerInside? false))

(event Custom|Victory
  ;[0.05098 0.05098 0.05098] Finalizando a Partida
  (if (Variables|Default|GetPlayerInside?)
    (bind _returnvalue (UserInterface|CreateWidget "/Game/MinhasBluePrints/Hud/HUD_VICTORY.HUD_VICTORY_C"))
    (UserInterface|Viewport|AddtoViewport _returnvalue 0)
    (Game|SpawnActorfromClass "/Game/MinhasBluePrints/BP_Bloco.BP_Bloco_C" (Math|Transform|MakeTransform "7100.000000,634.000000,130.000000" "0.000000,-30.000000,0.000000" "1.000000,1.000000,1.000000") "Undefined" "MultiplyWithRoot" 0 0)
    (Audio|PlaySound2D "/Game/MinhasBluePrints/Sons/vitoria.vitoria" 1.0 1.0 0.0 0 0)
    (bind _foundwidgets (Widget|GetAllWidgetsOfClass "/Game/MinhasBluePrints/Hud/HUD_ItemKey.HUD_ItemKey_C" true))
    (Widget|RemovefromParent _foundwidgets)
    (Variables|/Game/ThirdPerson/Blueprints/BP_ThirdPersonCharacter.BP_ThirdPersonCharacter_C|SetIsEnemy? (Variables|Default|GetPlayer%20Ref) false)
    (Utilities|FlowControl|Delay 5.3)
    (Actor|DestroyActor (Variables|Default|GetPlayer%20Ref))
    (Game|OpenLevel(byName) "L_Menu")))

(fn ConstructionScript)