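; Goose ("Ganso") enemy AI that chases the player and shoots on sight.
; BeginPlay caches the third-person character, and Tick refreshes its location as the move target.
; PawnSensing sightings start AI MoveTo, turn the goose's yaw toward the player, then after a short delay spawn BP_Tiro from an arrow with a sound.
; ApplyDamage fires when the move is issued, not on arrival, with no damage amount set.
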(event OnSeePawn(PawnSensing)
  (params (Pawn :type Pawn%20Object%20Reference))
  (CallFunction|MovetoPlayer)
  (Transformation|SetActorRotation (Math|Rotator|MakeRotator 0.0 0.0 (.yaw (Math|Rotator|FindLookatRotation (Transformation|GetActorLocation) (Transformation|GetActorLocation (Variables|Default|GetPlayerRef))))))
  (Utilities|FlowControl|Delay 0.7)
  (Game|SpawnActorfromClass "/Game/MinhasBluePrints/Emimes/BP_Tiro.BP_Tiro_C" (Transformation|GetWorldTransform (Variables|Default|GetArrow1)) "Undefined" "MultiplyWithRoot" 0 0)
  (Audio|PlaySound2D "/Game/MinhasBluePrints/Sons/ganso1.ganso1" 1.0 1.0 0.0 0 0))

(event Custom|Get%20player%20Position
  (Variables|Default|SetPlayerPosition (Transformation|GetActorLocation (Variables|Default|GetPlayerRef))))

(event Custom|MovetoPlayer
  ;[1 1 1] Move to Player
  (AI|AIMoveTo self (Variables|Default|GetPlayerPosition) (Variables|Default|GetPlayerRef) 5.0 false
    (:then
      (Game|Damage|ApplyDamage (Variables|Default|GetPlayerRef) 0.0 0 0))))

(event EventBeginPlay
  ;[1 1 1] Variavel do Player
  (bind _asbp_third_person_character (Utilities|Casting|CastToBP_ThirdPersonCharacter (Game|GetPlayerCharacter 0)))
  (Variables|Default|SetPlayerRef _asbp_third_person_character))

(event EventTick
  (params (DeltaSeconds :type Float%20%28single-precision%29))
  ;[1 1 1] GetPlayer Position
  (CallFunction|GetPlayerPosition))

(fn ConstructionScript)