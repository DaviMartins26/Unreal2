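; Goose enemy AI that acts as a following turret, shooting at and chasing the player when the player's IsEnemy flag is set.
; Caches the player character on BeginPlay and refreshes its location every Tick.
; PawnSensing sightings turn its yaw toward the player, then after a delay spawn a BP_TiroFloower projectile from an arrow, play a sound and start AIMoveTo.
; A successful move calls ApplyDamage on the player.
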(event OnSeePawn(PawnSensing)
  (params (Pawn :type Pawn%20Object%20Reference))
  ;[1 1 1] Tiro e Movimento
  (if (Variables|/Game/ThirdPerson/Blueprints/BP_ThirdPersonCharacter.BP_ThirdPersonCharacter_C|GetIsEnemy? (Variables|Default|GetPlayerRef))
    (Transformation|SetActorRotation (Math|Rotator|MakeRotator 0.0 0.0 (.yaw (Math|Rotator|FindLookatRotation (Transformation|GetActorLocation) (Transformation|GetActorLocation (Variables|Default|GetPlayerRef))))))
    (Utilities|FlowControl|Delay 1.5)
    (Game|SpawnActorfromClass "/Game/MinhasBluePrints/Emimes/BP_TiroFloower.BP_TiroFloower_C" (Transformation|GetWorldTransform (Variables|Default|GetArrow1)) "Undefined" "MultiplyWithRoot" 0 0)
    (Audio|PlaySound2D "/Game/MinhasBluePrints/Sons/ganso1.ganso1" 1.0 1.0 0.0 0 0)
    (CallFunction|MovetoPlayer)))

(event Custom|Get%20player%20Position
  ;[1 1 1] GetPosition
  (Variables|Default|SetPlayerPosition (Transformation|GetActorLocation (Variables|Default|GetPlayerRef))))

(event Custom|MovetoPlayer
  ;[1 1 1] Move to Player
  (if (Variables|/Game/ThirdPerson/Blueprints/BP_ThirdPersonCharacter.BP_ThirdPersonCharacter_C|GetIsEnemy? (Variables|Default|GetPlayerRef))
    (AI|AIMoveTo self (Variables|Default|GetPlayerPosition) (Variables|Default|GetPlayerRef) 3e+01 false
      (:OnSuccess
        (Game|Damage|ApplyDamage (Variables|Default|GetPlayerRef) 0.0 0 0)))))

(event EventBeginPlay
  ;[1 1 1] Variavel do Player
  (bind _asbp_third_person_character (Utilities|Casting|CastToBP_ThirdPersonCharacter (Game|GetPlayerCharacter 0)))
  (Variables|Default|SetPlayerRef _asbp_third_person_character))

(event EventTick
  (params (DeltaSeconds :type Float%20%28single-precision%29))
  ;[1 1 1] GetPlayer Position
  (CallFunction|GetPlayerPosition))

(fn ConstructionScript)