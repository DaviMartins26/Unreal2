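; BP_GansoTorreta is a goose turret that turns toward and shoots at a sighted third-person character whose IsEnemy flag is set.
; PawnSensing triggers the logic, snapping the actor's yaw toward that character.
; After a short Delay, which also paces repeated sightings, it spawns a BP_Tiro projectile at its Arrow's transform and plays a goose sound in 2D.
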(event OnSeePawn(PawnSensing)
  (params (Pawn :type Pawn%20Object%20Reference))
  ;[1 1 1] Tiro e movimento
  (bind _asbp_third_person_character (Utilities|Casting|CastToBP_ThirdPersonCharacter Pawn))
  (if (Variables|/Game/ThirdPerson/Blueprints/BP_ThirdPersonCharacter.BP_ThirdPersonCharacter_C|GetIsEnemy? _asbp_third_person_character)
    (Transformation|SetActorRotation (Math|Rotator|MakeRotator 0.0 0.0 (.yaw (Math|Rotator|FindLookatRotation (Transformation|GetActorLocation) (Transformation|GetActorLocation Pawn)))))
    (Utilities|FlowControl|Delay 0.6)
    (Game|SpawnActorfromClass "/Game/MinhasBluePrints/Emimes/BP_Tiro.BP_Tiro_C" (Transformation|GetWorldTransform (Variables|Default|GetArrow)) "Undefined" "MultiplyWithRoot" 0 0)
    (Audio|PlaySound2D "/Game/MinhasBluePrints/Sons/ganso1.ganso1" 1.0 1.0 0.0 0 0)))

(fn ConstructionScript)